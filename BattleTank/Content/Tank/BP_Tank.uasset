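; BP_Tank is a tank Blueprint with an orbiting aim camera driven by player input.
; On BeginPlay it hands its Barrel and Turret components to SetBarrelReference and SetTurretReference.
; The AimHorizontal axis yaws HorizontalGimbal and AimVertical pitches the SpringArm, both as local rotations scaled by delta time, keeping the two camera axes on separate components.
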(event `self.ReceiveBeginPlay`
  (`self.SetBarrelReference` (`self.Barrel`))
  (`self.SetTurretReference` (`self.Turret`)))

(event `InputAxis|AimHorizontal`
  (params (AxisValue :type "Float (single-precision)"))
  ;[1 1 1] Rotate the Camera
  (`SceneComponent.K2_AddLocalRotation` (`self.Horizontal Gimbal`) (`KismetMathLibrary.MakeRotator` 0.0 0.0 (* AxisValue (`GameplayStatics.GetWorldDeltaSeconds`) 100.0)) false false))

(event `InputAxis|AimVertical`
  (params (AxisValue :type "Float (single-precision)"))
  ;[1 1 1] Rotate the Camera
  (`SceneComponent.K2_AddLocalRotation` (`self.SpringArm`) (`KismetMathLibrary.MakeRotator` 0.0 (* AxisValue (`GameplayStatics.GetWorldDeltaSeconds`) 100.0)) false false))

(fn `UserConstructionScript`)